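; Cooking station that cooks overlapping ingredient actors into their CooksInto data, with a frying pan and camera-facing progress bar.
; DetectArea toggles pan and bar visibility, while CookingArea snaps one cookable ingredient in place and starts audio.
; Tick accumulates cook time on the ingredient itself, then swaps its data and re-enables physics.
; A hardcoded check for burnt patty results switches the frying sound and the bar's burn warning.
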(event `self.ReceiveBeginPlay`
  (`self.SetCookingTimerBar`)
  (`self.ToggleFryingPan` false))

(event `self.ReceiveTick`
  (params (DeltaSeconds :type "Float (single-precision)"))
  (bind _cookingloop (`self.CookingLoop`))
  (bind _currentcookingitem (`self.CurrentCookingItem`))
  (bind _itemdata (`/Game/BP_Interactable_Ingredient_Actor.ItemData` _currentcookingitem))
  (bind _cooktimetracked (`/Game/BP_Interactable_Ingredient_Actor.CookTimeTracked` _currentcookingitem))
  (bind _cooksinto (`/Game/PP_Items/DA_Item_Data.CooksInto` _itemdata))
  (bind _cooksinto_2 (`/Game/PP_Items/DA_Item_Data.CooksInto` (`/Game/BP_Interactable_Ingredient_Actor.ItemData` _currentcookingitem)))
  (`SceneComponent.K2_SetWorldRotation` (`self.CookingTimerWidget`) (`KismetMathLibrary.FindLookAtRotation` (`self.K2_GetActorLocation` self) (`PlayerCameraManager.GetCameraLocation` (`GameplayStatics.GetPlayerCameraManager` 0))) false false)
  (`/Engine/EditorBlueprintResources/StandardMacros.IsValid` _currentcookingitem
    (:`Is Valid`
      (`/Engine/EditorBlueprintResources/StandardMacros.IsValid` _cooksinto
        (:`Is Valid`
          (if (or (== _cooksinto "/Game/PP_Items/Item_Data_Patty_Burnt.Item_Data_Patty_Burnt") (== _cooksinto "/Game/PP_Items/Item_Data_Veggie_Patty_Burnt.Item_Data_Veggie_Patty_Burnt"))
            (set `self.CookingLoop` 1)
            (else
              (set `self.CookingLoop` 0)))
          (if (< _cooktimetracked (`/Game/PP_Items/DA_Item_Data.CookTime` _itemdata))
            (bind _output_get (set `/Game/BP_Interactable_Ingredient_Actor.CookTimeTracked` (+ _cooktimetracked DeltaSeconds) _currentcookingitem))
            (`self.UpdateCookingTimerBar` _output_get (`/Game/PP_Items/DA_Item_Data.CookTime` (`/Game/BP_Interactable_Ingredient_Actor.ItemData` _currentcookingitem)))
            (`AudioComponent.SetIntParameter` (`self.CookingAudio`) "Frying Sound File" _cookingloop)
            (bind _cooking_progress_bar (`self.GetCookingTimerBar`))
            (set `/Game/Cooking_Area/W_Cooking_Progress_Bar.WillBurn` (> _cookingloop 0) _cooking_progress_bar)
            (else
              (`/Engine/EditorBlueprintResources/StandardMacros.IsValid` _cooksinto_2
                (:`Is Valid`
                  (`/Game/BP_Interactable_Ingredient_Actor.ChangeData` _currentcookingitem _cooksinto_2)
                  (`PrimitiveComponent.SetSimulatePhysics` (`StaticMeshActor.StaticMeshComponent` _currentcookingitem) true)
                  (set `/Game/BP_Interactable_Ingredient_Actor.CookTimeTracked` 0.0 (`self.CurrentCookingItem`)))
                (:`Is Not Valid`
                  (`self.StoppedCooking` :!label _label))))))
        (:`Is Not Valid`
          (if (`AudioComponent.IsPlaying` (`self.CookingAudio`)) :!label _label_2
            (goto _label)))))
    (:`Is Not Valid`
      (goto _label_2))))

(event `StoppedCooking`
  (`AudioComponent.Stop` (`self.CookingAudio`)))

(event `StartedCooking`
  (`AudioComponent.Play` (`self.CookingAudio`) 0.0))

(event `self.CookingArea.OnComponentBeginOverlap`
  (params (OverlappedComponent :type "PrimitiveComponent Object Reference") (OtherActor :type "Actor Object Reference") (OtherComp :type "PrimitiveComponent Object Reference") (OtherBodyIndex :type Integer) (bFromSweep :type Boolean) (SweepResult :type "HitResult Structure (by ref)"))
  (`/Engine/EditorBlueprintResources/StandardMacros.IsValid` (`self.CurrentCookingItem`)
    (:`Is Not Valid`
      (if (`self.Is Actor An Ingredient` OtherActor)
        (bind _asbp_interactable_ingredient_actor (cast `/Game/BP_Interactable_Ingredient_Actor` OtherActor))
        (`/Engine/EditorBlueprintResources/StandardMacros.IsValid` _asbp_interactable_ingredient_actor
          (:`Is Valid`
            (`/Engine/EditorBlueprintResources/StandardMacros.IsValid` (`/Game/PP_Items/DA_Item_Data.CooksInto` (`/Game/BP_Interactable_Ingredient_Actor.ItemData` _asbp_interactable_ingredient_actor))
              (:`Is Valid`
                (bind _output_get (set `self.CurrentCookingItem` _asbp_interactable_ingredient_actor))
                (`PrimitiveComponent.SetSimulatePhysics` (`StaticMeshActor.StaticMeshComponent` _output_get) false)
                (`self.K2_SetActorLocationAndRotation` :`self` _output_get :`NewLocation` (`SceneComponent.K2_GetComponentLocation` (`self.CookingArea`)) :`bTeleport` true)
                (`self.StartedCooking`)))))))))

(event `self.CookingArea.OnComponentEndOverlap`
  (params (OverlappedComponent :type "PrimitiveComponent Object Reference") (OtherActor :type "Actor Object Reference") (OtherComp :type "PrimitiveComponent Object Reference") (OtherBodyIndex :type Integer))
  (bind _currentcookingitem (`self.CurrentCookingItem`))
  (if (`self.Is Actor An Ingredient` OtherActor)
    (bind _asbp_interactable_ingredient_actor (cast `/Game/BP_Interactable_Ingredient_Actor` OtherActor))
    (`/Engine/EditorBlueprintResources/StandardMacros.IsValid` _currentcookingitem
      (:`Is Valid`
        (if (== _asbp_interactable_ingredient_actor _currentcookingitem)
          (set `self.CurrentCookingItem` null)
          (`self.StoppedCooking` :!label _label_3)))
      (:`Is Not Valid`
        (`/Engine/EditorBlueprintResources/StandardMacros.IsValid` (`/Game/PP_Items/DA_Item_Data.CooksInto` (`/Game/BP_Interactable_Ingredient_Actor.ItemData` _asbp_interactable_ingredient_actor))
          (:`Is Valid`
            (set `self.CurrentCookingItem` _asbp_interactable_ingredient_actor))
          (:`Is Not Valid`
            (`self.ToggleFryingPan` false)
            (goto _label_3)))))))

(event `self.DetectArea.OnComponentBeginOverlap`
  (params (OverlappedComponent :type "PrimitiveComponent Object Reference") (OtherActor :type "Actor Object Reference") (OtherComp :type "PrimitiveComponent Object Reference") (OtherBodyIndex :type Integer) (bFromSweep :type Boolean) (SweepResult :type "HitResult Structure (by ref)"))
  (if (`self.Is Actor An Ingredient` OtherActor)
    (bind _asbp_interactable_ingredient_actor (cast `/Game/BP_Interactable_Ingredient_Actor` OtherActor))
    (`/Engine/EditorBlueprintResources/StandardMacros.IsValid` (`/Game/PP_Items/DA_Item_Data.CooksInto` (`/Game/BP_Interactable_Ingredient_Actor.ItemData` _asbp_interactable_ingredient_actor))
      (:`Is Valid`
        (`self.ToggleFryingPan` true))
      (:`Is Not Valid`
        (`self.ToggleFryingPan` false)))))

(event `self.DetectArea.OnComponentEndOverlap`
  (params (OverlappedComponent :type "PrimitiveComponent Object Reference") (OtherActor :type "Actor Object Reference") (OtherComp :type "PrimitiveComponent Object Reference") (OtherBodyIndex :type Integer))
  (bind _currentcookingitem (`self.CurrentCookingItem`))
  (if (`self.Is Actor An Ingredient` OtherActor)
    (bind _asbp_interactable_ingredient_actor (cast `/Game/BP_Interactable_Ingredient_Actor` OtherActor))
    (`/Engine/EditorBlueprintResources/StandardMacros.IsValid` _currentcookingitem
      (:`Is Valid`
        (if (== _currentcookingitem _asbp_interactable_ingredient_actor)
          (`self.ToggleFryingPan` false)))
      (:`Is Not Valid`
        (`self.ToggleFryingPan` false)))))

(fn `GetCookingTimerBar`
  (returns (`Cooking Progress Bar` :type "/Game/Cooking_Area/W_Cooking_Progress_Bar Object Reference"))
  (return (`self.Cooking Progress Bar`)))

(fn `Is Actor An Ingredient`
  (params (Actor :type "Actor Object Reference"))
  (returns (Result :type Boolean))
  (return (== (`GameplayStatics.GetObjectClass` Actor) "/Game/BP_Interactable_Ingredient_Actor.BP_Interactable_Ingredient_Actor_C")))

(fn `SetCookingTimerBar`
  (bind _asw_cooking_progress_bar (cast `/Game/Cooking_Area/W_Cooking_Progress_Bar` (`WidgetComponent.GetWidget` (`self.CookingTimerWidget`))))
  (set `self.Cooking Progress Bar` _asw_cooking_progress_bar))

(fn `ToggleFryingPan`
  (params (Visible :type Boolean))
  (`SceneComponent.SetVisibility` (`self.FryingPan`) Visible false)
  (`SceneComponent.SetVisibility` (`self.CookingTimerWidget`) Visible false))

(fn `UpdateCookingTimerBar`
  (params (TrackedTime :type "Float (double-precision)") (MaxTime :type "Float (double-precision)"))
  (bind _cooking_progress_bar (`self.Cooking Progress Bar`))
  (bind _output_get (set `/Game/Cooking_Area/W_Cooking_Progress_Bar.CookTime` TrackedTime _cooking_progress_bar))
  (bind _output_get_2 (set `/Game/Cooking_Area/W_Cooking_Progress_Bar.MaxCookTime` MaxTime _cooking_progress_bar))
  (`ProgressBar.SetPercent` (`/Game/Cooking_Area/W_Cooking_Progress_Bar.ProgressBar` _cooking_progress_bar) (`KismetMathLibrary.NormalizeToRange` _output_get 0.0 _output_get_2)))

(fn `UserConstructionScript`)