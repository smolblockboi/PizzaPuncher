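; A fridge item source that supplies ingredient actors on three shelves, with a door that swings open and shut when punched.
; BeginPlay fills each shelf to the shelf limit from its item data entry and sets the contents icon from the first item's material.
; Closing the door spawns one item on each shelf whose box overlap count is below the limit.
; Items spawn at random points within their shelf's box.
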(event `SpawnTopShelfItem`
  (`|SpawnActorFromClass` "/Game/BP_Interactable_Ingredient_Actor.BP_Interactable_Ingredient_Actor_C" (`self.GetFridgeSpawnTransform` 0) "AdjustIfPossibleButAlwaysSpawn" "MultiplyWithRoot" null (`|GetArrayItem` (`self.ItemSpawnData`) 0) null))

(event `SpawnMiddleShelfItem`
  (`|SpawnActorFromClass` "/Game/BP_Interactable_Ingredient_Actor.BP_Interactable_Ingredient_Actor_C" (`self.GetFridgeSpawnTransform` 1) "AdjustIfPossibleButAlwaysSpawn" "MultiplyWithRoot" null (`|GetArrayItem` (`self.ItemSpawnData`) 1) null))

(event `SpawnBottomShelfItem`
  (`|SpawnActorFromClass` "/Game/BP_Interactable_Ingredient_Actor.BP_Interactable_Ingredient_Actor_C" (`self.GetFridgeSpawnTransform` 2) "AdjustIfPossibleButAlwaysSpawn" "MultiplyWithRoot" null (`|GetArrayItem` (`self.ItemSpawnData`) 2) null))

(event `CloseDoor`
  (`SceneComponent.K2_SetRelativeRotation` :`self` (`self.DoorHinge`)))

(event `self.ReceiveBeginPlay`
  (set `self.ItemSpawnPoints` (`|MakeArray` (`self.ItemSpawnBoxTop`) (`self.ItemSpawnBoxMiddle`) (`self.ItemSpawnBoxBottom`)))
  (for _ (range (`self.ShelfLimit`))
    (for (_array_element _array_index) (`self.ItemSpawnData`)
      (`|SpawnActorFromClass` "/Game/BP_Interactable_Ingredient_Actor.BP_Interactable_Ingredient_Actor_C" (`self.GetFridgeSpawnTransform` _array_index) "AdjustIfPossibleButAlwaysSpawn" "MultiplyWithRoot" null _array_element null))
    (`PrimitiveComponent.SetMaterial` (`self.ContentsIcon`) 0 (`/Game/PP_Items/DA_Item_Data.ItemMaterial` (`|GetArrayItem` (`self.ItemSpawnData`))))))

(event `OpenDoor`
  (`SceneComponent.K2_SetRelativeRotation` (`self.DoorHinge`) (struct :`Yaw` -110.0) false false))

(event `self.GetPunched`
  (params (HitComponent :type "PrimitiveComponent Object Reference"))
  (bind _result (`self.GetShelfLimit`))
  (if (== (`self.DoorMesh`) HitComponent)
    (if (`self.IsClosed`)
      (`self.OpenDoor`)
      (set `self.IsClosed` false)
      (else
        (`self.CloseDoor`)
        (`|ExecutionSequence`
          (:`then_0`
            (bind _result_2 (`self.GetOverlapCount` (`self.ItemSpawnBoxTop`)))
            (if (< _result_2 _result)
              (`self.SpawnTopShelfItem`)))
          (:`then_1`
            (bind _result_3 (`self.GetOverlapCount` (`self.ItemSpawnBoxMiddle`)))
            (if (< _result_3 _result)
              (`self.SpawnMiddleShelfItem`)))
          (:`then_2`
            (bind _result_4 (`self.GetOverlapCount` (`self.ItemSpawnBoxBottom`)))
            (if (< _result_4 _result)
              (`self.SpawnBottomShelfItem`)))
          (:`then_3`
            (set `self.IsClosed` true)))))))

(fn `GetFridgeSpawnTransform`
  (params (ShelfIndex :type Integer))
  (returns (Result :type "Transform Structure"))
  (bind _output (`|GetArrayItem` (`self.ItemSpawnPoints`) ShelfIndex))
  (bind (_returnvalue_location _returnvalue_rotation _returnvalue_scale) (`KismetMathLibrary.BreakTransform` (`SceneComponent.K2_GetComponentToWorld` _output)))
  (return (`KismetMathLibrary.MakeTransform` (`KismetMathLibrary.RandomPointInBoundingBox` (`SceneComponent.K2_GetComponentLocation` _output) (`BoxComponent.GetScaledBoxExtent` _output)) _returnvalue_rotation _returnvalue_scale)))

(fn `GetOverlapCount`
  (params (Actor :type "PrimitiveComponent Object Reference"))
  (returns (Result :type Integer))
  (return (`KismetArrayLibrary.Array_Length` (`PrimitiveComponent.GetOverlappingActors` Actor null))))

(fn `GetShelfLimit`
  (returns (Result :type Integer))
  (return (`self.ShelfLimit`)))

(fn `UserConstructionScript`
  (`parent.UserConstructionScript`))