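; Game instance for a burger game that holds player money and ingredient unlock states, and gives access to the player HUD.
; Events add a value to the money total or broadcast an ingredient unlock through a dispatcher, without changing the unlock map here.
; Unlock checks look up the ingredient map by an item's SourceItem when valid, otherwise by the item itself.
; Helper functions return the first player's HUD and its UI reference.
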(event `/Game/HUD/BPI_Shop.IngredientUnlocked`
  (params (ItemData :type "/Game/PP_Items/DA_Item_Data Object Reference"))
  (`self.OnIngredientUnlocked` ItemData))

(event `ChangePlayerMoney`
  (params (Value :type Integer))
  (set `self.PlayerMoney` (+ Value (`self.PlayerMoney`))))

(fn `GetPlayerHUD`
  (returns (`Player HUD` :type "/Game/HUD/Player_HUD Object Reference"))
  (bind _asplayer_hud (cast `/Game/HUD/Player_HUD` (`PlayerController.GetHUD` (`GameplayStatics.GetPlayerController` 0))))
  (return _asplayer_hud))

(fn `GetPlayerUI_Ref`
  (returns (UI_Ref :type "/Game/HUD/BP_Player_Widget Object Reference"))
  (return (`/Game/HUD/Player_HUD.UI_Ref` (`self.GetPlayerHUD`))))

(fn `IsIngredientUnlocked`
  (params (ItemData :type "/Game/PP_Items/DA_Item_Data Object Reference"))
  (returns (Result :type Boolean))
  (bind _sourceitem (`/Game/PP_Items/DA_Item_Data.SourceItem` ItemData))
  (bind _burgeringredients (`self.BurgerIngredients`))
  (`/Engine/EditorBlueprintResources/StandardMacros.IsValid` _sourceitem
    (:`Is Valid`
      (return (`BlueprintMapLibrary.Map_Find` _burgeringredients _sourceitem)))
    (:`Is Not Valid`
      (return (`BlueprintMapLibrary.Map_Find` _burgeringredients ItemData)))))