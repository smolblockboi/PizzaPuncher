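; Item handler on the first-person character that lets the player grab, punch, chop and highlight objects in view.
; Camera line traces find targets, forwarding actions to BP_Interactable_Actor, while grabbed components follow a hold point through the character's PhysicsHandle.
; When nothing is held, Tick selects and deselects aimed-at actors through BP_Select_Interface.
; IA_Change_Hand swaps Punch and Chop input mapping contexts and signals the mode change.
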(event `self.ReceiveBeginPlay`
  ; Begin Play
  (bind _asbp_first_person_character (cast `/Game/FirstPerson/Blueprints/BP_FirstPersonCharacter` (`self.GetOwner`)))
  (bind _output_get (set `self.FirstPersonCharacter` _asbp_first_person_character))
  (bind _asplayer_controller (cast `PlayerController` (`Pawn.GetController` _output_get)))
  (bind _output_get_2 (set `self.PlayerController` _asplayer_controller))
  (bind _returnvalue (pcsubsystem `EnhancedInputLocalPlayerSubsystem` _output_get_2))
  (`/Engine/EditorBlueprintResources/StandardMacros.IsValid` _returnvalue
    (:`Is Valid`
      (`EnhancedInputSubsystemInterface.AddMappingContext` _returnvalue "/Game/PP_Input/IMC_Pizza_Puncher.IMC_Pizza_Puncher" 1 (struct))
      (`EnhancedInputSubsystemInterface.AddMappingContext` _returnvalue "/Game/PP_Input/IMC_Punch_Mode.IMC_Punch_Mode" 1 (struct)))))

(event `EnhancedInput|/Game/PP_Input/IA_Grab`
  (params (ActionValue :type Boolean) (ElapsedSeconds :type "Float (double-precision)") (TriggeredSeconds :type "Float (double-precision)") (InputAction :type "InputAction Object Reference" :default "/Game/PP_Input/IA_Grab.IA_Grab"))
  ; IA_Grab
  (:`Started`
    (`KismetSystemLibrary.PrintString` "Grabbed")
    (bind (_start _end) (`self.CameraLineTrace`))
    (bind (_outhit _returnvalue) (`KismetSystemLibrary.LineTraceSingle` :`Start` _start :`End` _end :`TraceChannel` "TraceTypeQuery1" :`DrawDebugType` "ForDuration"))
    (if _returnvalue
      (bind (_bblockinghit _binitialoverlap _time _distance _location _impactpoint _normal _impactnormal _physmat _hitactor _hitcomponent) (`GameplayStatics.BreakHitResult` _outhit))
      (`PhysicsHandleComponent.GrabComponentAtLocation` (`self.GetPlayerPhysicsHandle`) _hitcomponent "None" (`SceneComponent.K2_GetComponentLocation` _hitcomponent))
      (set `self.IsGrabbingObject` true)
      (bind _asbp_interactable_actor (cast `/Game/BP_Interactable_Actor` _hitactor))
      (bind _output_get (set `self.GrabbedActor` _asbp_interactable_actor))
      (`/Game/BP_Interactable_Actor.GetGrabbed` _output_get _hitcomponent)))
  (:`Completed`
    (`KismetSystemLibrary.PrintString` "Released")
    (`self.Let Go`)))

(event `EnhancedInput|/Game/PP_Input/IA_Punch`
  (params (ActionValue :type Boolean) (ElapsedSeconds :type "Float (double-precision)") (TriggeredSeconds :type "Float (double-precision)") (InputAction :type "InputAction Object Reference" :default "/Game/PP_Input/IA_Punch.IA_Punch"))
  ; IA_Punch
  (:`Triggered`
    (`KismetSystemLibrary.PrintString` "Punch")
    (bind (_start _end) (`self.CameraLineTrace`))
    (bind (_outhit _returnvalue) (`KismetSystemLibrary.LineTraceSingle` :`Start` _start :`End` _end :`TraceChannel` "TraceTypeQuery1" :`DrawDebugType` "ForDuration"))
    (if _returnvalue
      (bind (_bblockinghit _binitialoverlap _time _distance _location _impactpoint _normal _impactnormal _physmat _hitactor _hitcomponent) (`GameplayStatics.BreakHitResult` _outhit))
      (bind _asbp_interactable_actor (cast `/Game/BP_Interactable_Actor` _hitactor))
      (`/Game/BP_Interactable_Actor.GetPunched` _asbp_interactable_actor _hitcomponent))))

(event `self.ReceiveTick`
  (params (DeltaSeconds :type "Float (single-precision)"))
  (bind _selectedactor (`self.SelectedActor`))
  (bind _selectedactor_2 (`self.SelectedActor`))
  (if (`self.IsGrabbingObject`)
    (bind (_start _end) (`self.HoldLineTrace`))
    (`PhysicsHandleComponent.SetTargetLocation` (`self.GetPlayerPhysicsHandle`) _end)
    (else
      (bind (_start_2 _end_2) (`self.CameraLineTrace`))
      (bind (_outhit _returnvalue) (`KismetSystemLibrary.LineTraceSingleForObjects` _start_2 _end_2 (`|MakeArray` "ObjectTypeQuery4" "ObjectTypeQuery2" :!type "EObjectTypeQuery Enum")))
      (if _returnvalue
        (bind (_bblockinghit _binitialoverlap _time _distance _location _impactpoint _normal _impactnormal _physmat _hitactor) (`GameplayStatics.BreakHitResult` _outhit))
        (if (`KismetSystemLibrary.DoesImplementInterface` _hitactor "/Game/BP_Select_Interface.BP_Select_Interface_C")
          (bind _isselected (message `/Game/BP_Select_Interface.IsSelected` _hitactor))
          (if (not _isselected)
            (`/Engine/EditorBlueprintResources/StandardMacros.IsValid` _selectedactor
              (:`Is Valid`
                (message `/Game/BP_Select_Interface.DeselectActor` _selectedactor))
              (:`Is Not Valid`
                _))
            (message `/Game/BP_Select_Interface.SelectActor` _hitactor)
            (set `self.SelectedActor` _hitactor))
          (else
            (`/Engine/EditorBlueprintResources/StandardMacros.IsValid` _selectedactor_2 :!label _label
              (:`Is Valid`
                (message `/Game/BP_Select_Interface.DeselectActor` _selectedactor_2)
                (set `self.SelectedActor` null)))))
        (else
          (goto _label))))))

(event `EnhancedInput|/Game/PP_Input/IA_Chop`
  (params (ActionValue :type Boolean) (ElapsedSeconds :type "Float (double-precision)") (TriggeredSeconds :type "Float (double-precision)") (InputAction :type "InputAction Object Reference" :default "/Game/PP_Input/IA_Chop.IA_Chop"))
  ; IA_Chop
  (:`Triggered`
    (`KismetSystemLibrary.PrintString` "Chop")
    (bind (_start _end) (`self.CameraLineTrace`))
    (bind (_outhit _returnvalue) (`KismetSystemLibrary.LineTraceSingle` :`Start` _start :`End` _end :`TraceChannel` "TraceTypeQuery1" :`DrawDebugType` "ForDuration"))
    (if _returnvalue
      (bind (_bblockinghit _binitialoverlap _time _distance _location _impactpoint _normal _impactnormal _physmat _hitactor _hitcomponent) (`GameplayStatics.BreakHitResult` _outhit))
      (bind _asbp_interactable_actor (cast `/Game/BP_Interactable_Actor` _hitactor))
      (`/Game/BP_Interactable_Actor.GetChopped` _asbp_interactable_actor _hitcomponent))))

(event `Let Go`
  (`PhysicsHandleComponent.ReleaseComponent` (`self.GetPlayerPhysicsHandle`))
  (set `self.IsGrabbingObject` false)
  (set `self.GrabbedActor` null))

(event `EnhancedInput|/Game/PP_Input/IA_Change_Hand`
  (params (ActionValue :type "Float (double-precision)") (ElapsedSeconds :type "Float (double-precision)") (TriggeredSeconds :type "Float (double-precision)") (InputAction :type "InputAction Object Reference" :default "/Game/PP_Input/IA_Change_Hand.IA_Change_Hand"))
  (bind _returnvalue (pcsubsystem `EnhancedInputLocalPlayerSubsystem` (`self.PlayerController`)))
  ; Cycle Between Chop and Punch Modes
  (:`Triggered`
    (`/Engine/EditorBlueprintResources/StandardMacros.IsValid` _returnvalue
      (:`Is Valid`
        (if (< ActionValue 0.0)
          (`EnhancedInputSubsystemInterface.RemoveMappingContext` _returnvalue "/Game/PP_Input/IMC_Chop_Mode.IMC_Chop_Mode" (struct))
          (`EnhancedInputSubsystemInterface.AddMappingContext` _returnvalue "/Game/PP_Input/IMC_Punch_Mode.IMC_Punch_Mode" 1 (struct))
          (`KismetSystemLibrary.PrintString` "Changed to Punch mode")
          (`self.OnChangedActionMode` 0)
          (else
            (`EnhancedInputSubsystemInterface.RemoveMappingContext` _returnvalue "/Game/PP_Input/IMC_Punch_Mode.IMC_Punch_Mode" (struct))
            (`EnhancedInputSubsystemInterface.AddMappingContext` _returnvalue "/Game/PP_Input/IMC_Chop_Mode.IMC_Chop_Mode" 1 (struct))
            (`KismetSystemLibrary.PrintString` "Changed to Chop Mode")
            (`self.OnChangedActionMode` 1)))))))

(fn `CameraLineTrace`
  (returns (Start :type "Vector Structure") (End :type "Vector Structure"))
  (bind _transformcomponent (`PlayerCameraManager.TransformComponent` (`PlayerController.PlayerCameraManager` (`self.PlayerController`))))
  (bind _returnvalue (`SceneComponent.K2_GetComponentLocation` _transformcomponent))
  (return _returnvalue (+ _returnvalue (* (`KismetMathLibrary.GetForwardVector` (`SceneComponent.K2_GetComponentRotation` _transformcomponent)) (`self.GrabDistance`)))))

(fn `GetPlayerPhysicsHandle`
  (returns (PhysicsHandle :type "PhysicsHandleComponent Object Reference"))
  (return (`/Game/FirstPerson/Blueprints/BP_FirstPersonCharacter.PhysicsHandle` (`self.FirstPersonCharacter`))))

(fn `HoldLineTrace`
  (returns (Start :type "Vector Structure") (End :type "Vector Structure"))
  (bind _transformcomponent (`PlayerCameraManager.TransformComponent` (`PlayerController.PlayerCameraManager` (`self.PlayerController`))))
  (bind _returnvalue (`SceneComponent.K2_GetComponentLocation` _transformcomponent))
  (return _returnvalue (+ _returnvalue (* (`KismetMathLibrary.GetForwardVector` (`SceneComponent.K2_GetComponentRotation` _transformcomponent)) (`self.HoldDistance`)))))