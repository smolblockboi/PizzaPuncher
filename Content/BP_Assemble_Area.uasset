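; BP_Assemble_Area is a plate station where dropped ingredients are assembled into a food combo.
; When an ingredient actor overlaps its box, it adds the ingredient's item data to the current combo actor.
; With no valid combo, it spawns a new one atop the plate, offset by the mesh bounds height and seeded with that data.
; The ingredient actor is then destroyed.
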(event `self.Box.OnComponentBeginOverlap`
  (params (OverlappedComponent :type "PrimitiveComponent Object Reference") (OtherActor :type "Actor Object Reference") (OtherComp :type "PrimitiveComponent Object Reference") (OtherBodyIndex :type Integer) (bFromSweep :type Boolean) (SweepResult :type "HitResult Structure (by ref)"))
  (bind _plate (`self.Plate`))
  (bind (_min _max) (`StaticMeshComponent.GetLocalBounds` _plate))
  (bind (_returnvalue_location _returnvalue_rotation _returnvalue_scale) (`KismetMathLibrary.BreakTransform` (`SceneComponent.K2_GetComponentToWorld` _plate)))
  (bind (_returnvalue_x _returnvalue_y _returnvalue_z) (`KismetMathLibrary.BreakVector` (`SceneComponent.K2_GetComponentLocation` _plate)))
  (bind (_returnvalue_x_2 _returnvalue_y_2 _returnvalue_z_2) (`KismetMathLibrary.BreakVector` (- _max _min)))
  (if (== (`GameplayStatics.GetObjectClass` OtherActor) "/Game/BP_Interactable_Ingredient_Actor.BP_Interactable_Ingredient_Actor_C")
    (bind _asbp_interactable_ingredient_actor (cast `/Game/BP_Interactable_Ingredient_Actor` OtherActor))
    (`/Engine/EditorBlueprintResources/StandardMacros.IsValid` (`self.FoodComboActor`)
      (:`Is Valid`
        (`/Game/BP_Interactable_Food_Combo.AddItem` (`self.FoodComboActor`) (`/Game/BP_Interactable_Ingredient_Actor.ItemData` _asbp_interactable_ingredient_actor)))
      (:`Is Not Valid`
        (bind _returnvalue (`|SpawnActorFromClass` "/Game/BP_Interactable_Food_Combo.BP_Interactable_Food_Combo_C" (`KismetMathLibrary.MakeTransform` (`KismetMathLibrary.MakeVector` _returnvalue_x _returnvalue_y (+ _returnvalue_z _returnvalue_z_2)) _returnvalue_rotation _returnvalue_scale) "AdjustIfPossibleButAlwaysSpawn" "MultiplyWithRoot" null (`/Game/BP_Interactable_Ingredient_Actor.ItemData` _asbp_interactable_ingredient_actor) null))
        (set `self.FoodComboActor` _returnvalue)))
    (`/Engine/EditorBlueprintResources/StandardMacros.IsValid` _asbp_interactable_ingredient_actor
      (:`Is Valid`
        (`self.K2_DestroyActor` _asbp_interactable_ingredient_actor)))))

(fn `UserConstructionScript`)