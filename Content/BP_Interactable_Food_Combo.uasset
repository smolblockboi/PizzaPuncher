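; Interactable food combo that builds a visual stack from a base item plus ingredient actors dropped onto it.
; Capsule overlap absorbs and destroys ingredient actors, recording their item data and counting contaminated ones.
; Each ingredient becomes a new non-physics mesh component, stacked using the previous mesh's bounds and height offset, with outline overlay and sound.
; Contaminated pieces get a dynamic material with the Contamination parameter set.
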(event `AddIngredient`
  (params (ItemActor :type "/Game/BP_Interactable_Ingredient_Actor Object Reference") (ItemData :type "/Game/PP_Items/DA_Item_Data Object Reference") (IsContaminated :type Boolean))
  (bind _ingredientitemdata (`self.IngredientItemData`))
  (`/Engine/EditorBlueprintResources/StandardMacros.IsValid` ItemActor
    (:`Is Valid`
      (set `self.IngredientItemData` (`/Game/BP_Interactable_Ingredient_Actor.ItemData` ItemActor)))
    (:`Is Not Valid`
      (set `self.IngredientItemData` ItemData)))
  (`KismetArrayLibrary.Array_Add` (`self.ItemDatas`) _ingredientitemdata)
  (bind _zoffset (`self.GetLastMeshOffset`))
  (bind _returnvalue (`AddComponent|NODE_AddStaticMeshComponent-0` :`RelativeTransform` (`KismetMathLibrary.MakeTransform` (`KismetMathLibrary.MakeVector` 0.0 0.0 _zoffset))))
  (`|ExecutionSequence`
    (:`then_0`
      (set `self.LastMeshHeightOffset` (`/Game/PP_Items/DA_Item_Data.HeightOffset` _ingredientitemdata))
      (bind _output_get (set `self.LastMeshAdded` _returnvalue))
      (`MeshComponent.SetOverlayMaterial` _output_get (`self.OutlineMaterial`))
      (set `PrimitiveComponent.bGenerateOverlapEvents` false _output_get)
      (`PrimitiveComponent.SetSimulatePhysics` _output_get false)
      (`StaticMeshComponent.SetStaticMesh` _output_get (`/Game/PP_Items/DA_Item_Data.ItemMesh` _ingredientitemdata))
      (`AudioComponent.Play` (`self.AddIngredientAudio`) 0.0))
    (:`then_1`
      (if IsContaminated
        (bind _returnvalue_2 (`PrimitiveComponent.CreateDynamicMaterialInstance` _returnvalue 0 (`PrimitiveComponent.GetMaterial` _returnvalue 0) "None"))
        (`PrimitiveComponent.SetMaterial` _returnvalue 0 _returnvalue_2)
        (`MaterialInstanceDynamic.SetScalarParameterValue` _returnvalue_2 "Contamination" 1.0)))))

(event `self.Capsule.OnComponentBeginOverlap`
  (params (OverlappedComponent :type "PrimitiveComponent Object Reference") (OtherActor :type "Actor Object Reference") (OtherComp :type "PrimitiveComponent Object Reference") (OtherBodyIndex :type Integer) (bFromSweep :type Boolean) (SweepResult :type "HitResult Structure (by ref)"))
  (if (== (`GameplayStatics.GetObjectClass` OtherActor) "/Game/BP_Interactable_Ingredient_Actor.BP_Interactable_Ingredient_Actor_C")
    (bind _asbp_interactable_ingredient_actor (cast `/Game/BP_Interactable_Ingredient_Actor` OtherActor))
    (bind _iscontaminated (`/Game/BP_Interactable_Ingredient_Actor.IsContaminated` _asbp_interactable_ingredient_actor))
    (if _iscontaminated
      (`/Engine/EditorBlueprintResources/StandardMacros.IncrementInt` (`self.ContaminatedCount`)
        (:`  `
          _)))
    (`self.AddIngredient` _asbp_interactable_ingredient_actor null _iscontaminated)
    (`self.K2_DestroyActor` _asbp_interactable_ingredient_actor)))

(fn `GetLastMeshOffset`
  (returns (ZOffset :type "Float (double-precision)"))
  (bind _lastmeshadded (`self.LastMeshAdded`))
  (bind (_min _max) (`StaticMeshComponent.GetLocalBounds` (`self.StaticMeshComponent`)))
  (bind (_min_2 _max_2) (`StaticMeshComponent.GetLocalBounds` _lastmeshadded))
  (bind (_relativelocation_x _relativelocation_y _relativelocation_z) (`KismetMathLibrary.BreakVector` (`SceneComponent.RelativeLocation` _lastmeshadded)))
  (`/Engine/EditorBlueprintResources/StandardMacros.IsValid` _lastmeshadded
    (:`Is Valid`
      (return (- (+ _relativelocation_z (- (.z _max_2) (.z _min_2))) (`self.LastMeshHeightOffset`))))
    (:`Is Not Valid`
      (return (- (.z _max) (.z _min))))))

(fn `UserConstructionScript`
  (`parent.UserConstructionScript`)
  (`self.AddIngredient` null (`self.BaseItemData`) (`self.BaseItemContaminated`))
  (`AudioComponent.Play` (`self.AddIngredientAudio`) 0.0))