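; Interactable shop actor for the burger game that opens the shop menu when grabbed.
; OpenShopMenu creates BP_Shop_Widget, stores it on the game instance, switches input to UI only and centers a visible cursor.
; The widget's close button is bound to CloseShop, which removes the widget and restores game-only input.
; Opening and closing both play the same shop audio; NewMacro is an unused duplicate of the open logic.
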(event `self.GetGrabbed`
  (params (HitComponent :type "PrimitiveComponent Object Reference"))
  (bind _close_button (`self.OpenShopMenu`))
  (add `Button.OnPressed` _close_button (delegate `CloseShop`))
  (`AudioComponent.Play` (`self.ShopOpenAudio`) 0.0 :!label _label))

(event `CloseShop`
  (`self.CloseShopMenu`)
  (goto _label))

(fn `CloseShopMenu`
  (bind _returnvalue (`GameplayStatics.GetPlayerController` 0))
  (bind _asbp_burger_game_instance (cast `/Game/BP_Burger_Game_Instance` (`GameplayStatics.GetGameInstance`)))
  (`Widget.RemoveFromParent` (`/Game/BP_Burger_Game_Instance.OpenShopWidget` _asbp_burger_game_instance))
  (`WidgetBlueprintLibrary.SetInputMode_GameOnly` _returnvalue)
  (set `PlayerController.bShowMouseCursor` false _returnvalue))

(fn `OpenShopMenu`
  (returns (Close_Button :type "Button Object Reference"))
  (bind _returnvalue (`GameplayStatics.GetPlayerController` 0))
  (bind (_returnvalue_x _returnvalue_y) (`KismetMathLibrary.BreakVector2D` (/ (`WidgetLayoutLibrary.GetViewportSize`) (2.0 2.0))))
  (bind _returnvalue_2 (`|CreateWidget` "/Game/HUD/BP_Shop_Widget.BP_Shop_Widget_C" _returnvalue))
  (bind _asbp_burger_game_instance (cast `/Game/BP_Burger_Game_Instance` (`GameplayStatics.GetGameInstance`)))
  (bind _output_get (set `/Game/BP_Burger_Game_Instance.OpenShopWidget` _returnvalue_2 _asbp_burger_game_instance))
  (`UserWidget.AddToViewport` _output_get 0)
  (`WidgetBlueprintLibrary.SetInputMode_UIOnlyEx` _returnvalue _output_get)
  (set `PlayerController.bShowMouseCursor` true _returnvalue)
  (`PlayerController.SetMouseLocation` _returnvalue (`KismetMathLibrary.FTrunc` _returnvalue_x) (`KismetMathLibrary.FTrunc` _returnvalue_y))
  (return (`/Game/HUD/BP_Shop_Widget.Close_Button` _output_get)))

(fn `UserConstructionScript`
  (`parent.UserConstructionScript`))