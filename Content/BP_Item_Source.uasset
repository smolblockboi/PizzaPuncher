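; Item source actor that dispenses ingredient actors into the world when it receives its GetGrabbed event.
; SpawnItems creates one BP_Interactable_Ingredient_Actor per valid ItemSpawnData entry, passing that entry as its item data, then SpawnAudio plays.
; All items target the same point, a fixed distance along SpawnVector rotated into the actor's orientation, relying on collision adjustment while always spawning.
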(event `self.GetGrabbed`
  (params (HitComponent :type "PrimitiveComponent Object Reference"))
  (`self.SpawnItems`)
  (`AudioComponent.Play` (`self.SpawnAudio`) 0.0))

(fn `SpawnItems`
  (bind (_returnvalue_location _returnvalue_rotation) (`KismetMathLibrary.BreakTransform` (`self.GetTransform`)))
  (for _array_element (`self.ItemSpawnData`)
    (`/Engine/EditorBlueprintResources/StandardMacros.IsValid` _array_element
      (:`Is Valid`
        (`|SpawnActorFromClass` "/Game/BP_Interactable_Ingredient_Actor.BP_Interactable_Ingredient_Actor_C" (`KismetMathLibrary.MakeTransform` (+ _returnvalue_location (* (`KismetMathLibrary.GreaterGreater_VectorRotator` (`self.SpawnVector`) _returnvalue_rotation) 150.0))) "AdjustIfPossibleButAlwaysSpawn" "MultiplyWithRoot" null _array_element null)))))

(fn `UserConstructionScript`
  (`parent.UserConstructionScript`))