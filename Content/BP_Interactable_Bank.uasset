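; BP_Interactable_Bank is a debug interactable that gives the player money when grabbed.
; The grab event plays a cash register sound and adds a fixed amount through the game instance's ChangePlayerMoney.
; On the child begin-play event it checks the build configuration and destroys itself in Shipping builds, so it only exists in non-shipping builds.
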(event `self.ChildBeginPlay`
  (if (== (`KismetSystemLibrary.GetBuildConfiguration`) "Shipping")
    (`self.K2_DestroyActor`)))

(event `self.GetGrabbed`
  (params (HitComponent :type "PrimitiveComponent Object Reference"))
  (bind _burger_game_instance (`/Game/BP_Burger_Function_Library.GetGameInstance` self))
  (`GameplayStatics.PlaySound2D` "/Game/Order_Bell/201159__kiddpark__cash-register.201159__kiddpark__cash-register" 1.0 1.0 0.0 null null)
  (`/Game/BP_Burger_Game_Instance.ChangePlayerMoney` _burger_game_instance 100))

(fn `UserConstructionScript`
  (`parent.UserConstructionScript`))