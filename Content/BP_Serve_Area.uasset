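; BP_Serve_Area is the burger order counter: it generates orders and judges food combos dropped into its box.
; AddNewOrder builds a recipe from a template, filtering locked ingredients and randomizing the rest, then updates icon meshes and, via dispatcher, the active orders and HUD slips.
; On overlap, it compares the combo's items in order against active orders and destroys it.
; A match removes the order and, unless it is free, spawns money valued by matched ingredients.
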(event `AddNewOrder`
  (`self.ChangeToNewRecipe`))

(event `self.ReceiveBeginPlay`
  (`KismetSystemLibrary.Delay` 0.1)
  (bind _burger_game_instance (`/Game/BP_Burger_Function_Library.GetGameInstance` self))
  (set `/Game/BP_Burger_Game_Instance.OrderWindowBP` self _burger_game_instance)
  (bind _output_get (set `self.BP Burger Game Instance` _burger_game_instance))
  (set `self.Orders UI Ref` (`/Game/HUD/Player_HUD.Orders UI Ref` (`/Game/BP_Burger_Game_Instance.Player Hud Ref` _output_get)))
  (add `self.OnNewRecipeGenerated` (delegate `SendNewOrderToUI`))
  (add `self.OnOrderFulfilled` (delegate `RemoveOrderFromUI`))
  (for (_array_element _array_index) (`SceneComponent.GetChildrenComponents` (`self.IconsRoot`) false)
    (`SceneComponent.K2_AddRelativeLocation` _array_element (`KismetMathLibrary.MakeVector` 0.0 (`KismetMathLibrary.Conv_IntToDouble` (* _array_index -25))) false true)))

(event `SendNewOrderToUI`
  (bind _result (`/Engine/EditorBlueprintResources/StandardMacros.IncrementInt` (`self.TotalOrders`))
    (:`  `
      (bind _str_burger_order (make `/Game/PP_Recipes/STR_Burger_Order` _result (`self.TargetBurgerIngredients`)))
      (`/Game/HUD/Order_System/BP_Orders_Widget.MakeNewOrder` (`/Game/HUD/Player_HUD.Orders UI Ref` (`/Game/BP_Burger_Game_Instance.Player Hud Ref` (stale `self.ReceiveBeginPlay` _output_get))) _str_burger_order)
      (`KismetArrayLibrary.Array_Add` (`self.ActiveOrders`) _str_burger_order))))

(event `RemoveOrderFromUI` :!signature `self.OnOrderFulfilled`
  (params (OrderIndex :type Integer))
  (`/Game/HUD/Order_System/BP_Orders_Widget.RemoveOrder` (`/Game/HUD/Player_HUD.Orders UI Ref` (`/Game/BP_Burger_Game_Instance.Player Hud Ref` (stale `self.ReceiveBeginPlay` _output_get))) OrderIndex)
  (`KismetArrayLibrary.Array_Remove` (`self.ActiveOrders`) OrderIndex))

(event `self.Box.OnComponentBeginOverlap`
  (params (OverlappedComponent :type "PrimitiveComponent Object Reference") (OtherActor :type "Actor Object Reference") (OtherComp :type "PrimitiveComponent Object Reference") (OtherBodyIndex :type Integer) (bFromSweep :type Boolean) (SweepResult :type "HitResult Structure (by ref)"))
  (if (== (`GameplayStatics.GetObjectClass` OtherActor) "/Game/BP_Interactable_Food_Combo.BP_Interactable_Food_Combo_C")
    (bind _asbp_interactable_food_combo (cast `/Game/BP_Interactable_Food_Combo` OtherActor))
    (set `self.SubmittedFoodCombo` _asbp_interactable_food_combo)
    (for (_array_element _array_index) (`self.ActiveOrders`)
      (set `self.Matches` 0)
      (for (_array_element_2 _array_index_2) (`/Game/BP_Interactable_Food_Combo.ItemDatas` (`self.SubmittedFoodCombo`))
        (bind (_ordernumber _ingredients) (break `/Game/PP_Recipes/STR_Burger_Order` _array_element))
        (if (<= _array_index_2 (`KismetArrayLibrary.Array_Length` _ingredients))
          (if (== (`|GetArrayItem` _ingredients _array_index_2) _array_element_2)
            (bind _result (`/Engine/EditorBlueprintResources/StandardMacros.IncrementInt` (`self.Matches`))
              (:`  `
                (`KismetSystemLibrary.PrintString` (`KismetStringLibrary.Conv_IntToString` _result))))
            (else
              (break)))
          (else
            (break))))
      (`self.PrintServeResults` (`/Game/BP_Interactable_Food_Combo.ItemDatas` (`self.SubmittedFoodCombo`)) (`self.TargetBurgerIngredients`))
      (if (`self.MadeCorrectCombo` _ingredients)
        (`KismetSystemLibrary.PrintString` "CORRECT COMBO" true true (struct :`R` 0.083333 :`G` 1.0 :`A` 1.0))
        (break)
        (else
          (`KismetSystemLibrary.PrintString` "INCORRECT COMBO" true true (struct :`R` 1.0 :`A` 1.0)))))
    (bind _bp_burger_order_slip (`/Game/HUD/Order_System/BP_Orders_Widget.GetOrderSlip` (`self.Orders UI Ref`) _array_index))
    (`self.K2_DestroyActor` (`self.SubmittedFoodCombo`))
    (bind (_orderstruct_ordernumber _orderstruct_ingredients _orderstruct_iseatingforfree) (break `/Game/PP_Recipes/STR_Burger_Order` (`/Game/HUD/Order_System/BP_Burger_Order_Slip.OrderStruct` _bp_burger_order_slip)))
    ; did make correct combo?
    (if (`self.MadeCorrectCombo` _orderstruct_ingredients)
      ; is eating for free?
      (if (not _orderstruct_iseatingforfree)
        (`|SpawnActorFromClass` "/Game/BP_Interactable_Currency_Actor.BP_Interactable_Currency_Actor_C" (`SceneComponent.K2_GetComponentToWorld` (`self.MoneySpawner`)) "AdjustIfPossibleButAlwaysSpawn" "MultiplyWithRoot" null (`self.Matches`) null)
        (`AudioComponent.Play` (`self.Cash Sound`) 0.0))
      (`self.OnOrderFulfilled` _array_index))))

(fn `ChangeToNewRecipe`
  (locals (LocalChildIconMeshes :type "Array of SceneComponent Object Reference"))
  (`self.SetNewRandomRecipe`)
  (set `local.LocalChildIconMeshes` (`SceneComponent.GetChildrenComponents` (`self.IconsRoot`) false))
  (for _array_element (`local.LocalChildIconMeshes`)
    (`SceneComponent.SetHiddenInGame` _array_element true false))
  (for (_array_element_2 _array_index) (`self.TargetBurgerIngredients`)
    (bind _asstatic_mesh_component (cast `StaticMeshComponent` (`|GetArrayItem` (`local.LocalChildIconMeshes`) _array_index)))
    (bind _itemmaterial (`/Game/PP_Items/DA_Item_Data.ItemMaterial` _array_element_2))
    (`/Engine/EditorBlueprintResources/StandardMacros.IsValid` _itemmaterial
      (:`Is Valid`
        (`PrimitiveComponent.SetMaterial` _asstatic_mesh_component 0 _itemmaterial)
        (`SceneComponent.SetHiddenInGame` _asstatic_mesh_component false false))))
  (`self.OnNewRecipeGenerated`))

(fn `MadeCorrectCombo`
  (params (CheckedIngredients :type "Array of /Game/PP_Items/DA_Item_Data Object Reference"))
  (returns (ReturnValue :type Boolean))
  (return (== (`self.Matches`) (`KismetArrayLibrary.Array_Length` CheckedIngredients))))

(fn `PrintServeResults`
  (params (Submission :type "Array of /Game/PP_Items/DA_Item_Data Object Reference") (Target :type "Array of /Game/PP_Items/DA_Item_Data Object Reference"))
  (for _array_element Submission
    (`KismetSystemLibrary.PrintString` (`KismetSystemLibrary.GetDisplayName` _array_element) true true (struct :`R` 1.0 :`G` 0.843959 :`A` 1.0) 5.0))
  (for _array_element_2 Target
    (`KismetSystemLibrary.PrintString` (`KismetSystemLibrary.GetDisplayName` _array_element_2) true true (struct :`R` 1.0 :`B` 0.182753 :`A` 1.0) 5.0)))

(fn `SetNewRandomRecipe`
  (bind _targetburgeringredients (`self.TargetBurgerIngredients`))
  (`KismetArrayLibrary.Array_Clear` (`self.TargetBurgerIngredients`))
  (bind _output_get (set `self.TargetBurgerIngredients` (`/Game/PP_Recipes/DA_Food_Recipe.RequiredItems` (`self.BurgerTemplateData`))))
  (bind (_arrayindex _arrayelement) (`/Engine/EditorBlueprintResources/StandardMacros.ReverseForEachLoop` _output_get)
    (:`LoopBody`
      ; Remove Locked Ingredients
      (bind _result (`/Game/BP_Burger_Game_Instance.IsIngredientUnlocked` (`self.BP Burger Game Instance`) _arrayelement))
      (if (not _result)
        (`KismetArrayLibrary.Array_Remove` (`self.TargetBurgerIngredients`) _arrayindex)))
    (:`Completed`
      (for (_array_element _array_index) (`self.TargetBurgerIngredients`)
        ; Ingredient Variation
        (if (not (or (== _array_element "/Game/PP_Items/Item_Data_Bun_Bottom.Item_Data_Bun_Bottom") (== _array_element "/Game/PP_Items/Item_Data_Patty_Cooked.Item_Data_Patty_Cooked") (== _array_element "/Game/PP_Items/Item_Data_Bun_Top.Item_Data_Bun_Top")))
          (if (`KismetMathLibrary.RandomBool`)
            (`KismetArrayLibrary.Array_Remove` (`self.TargetBurgerIngredients`) _array_index))))
      ; Patty Generation
      (if (`KismetMathLibrary.RandomBool`)
        (`KismetArrayLibrary.Array_Set` _targetburgeringredients (`KismetArrayLibrary.Array_Find` _targetburgeringredients "/Game/PP_Items/Item_Data_Patty_Cooked.Item_Data_Patty_Cooked") "/Game/PP_Items/Item_Data_Veggie_Patty_Cooked.Item_Data_Veggie_Patty_Cooked")))))

(fn `UserConstructionScript`)