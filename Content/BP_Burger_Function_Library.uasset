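; Blueprint function library providing shared helper lookups for the burger game.
; It returns the game instance cast to BP_Burger_Game_Instance and player 0's HUD cast to Player_HUD.
; It also reports whether the build is Shipping by comparing the build configuration string to a literal.
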(fn `Get Player HUD`
  (params (WorldContextObject :type "Object Object Reference"))
  (returns (`AsPlayer HUD` :type "/Game/HUD/Player_HUD Object Reference"))
  (bind _asplayer_hud (cast `/Game/HUD/Player_HUD` (`PlayerController.GetHUD` (`GameplayStatics.GetPlayerController` WorldContextObject))))
  (return _asplayer_hud))

(fn `GetGameInstance`
  (params (WorldContextObject :type "Object Object Reference"))
  (returns (`Burger Game Instance` :type "/Game/BP_Burger_Game_Instance Object Reference"))
  (bind _asbp_burger_game_instance (cast `/Game/BP_Burger_Game_Instance` (`GameplayStatics.GetGameInstance` WorldContextObject))
    (:`then`
      (return _asbp_burger_game_instance))
    (:`CastFailed`
      (return null))))

(fn `Is Build Configuration Shipping`
  (returns (ReturnValue :type Boolean))
  (return (== (`KismetSystemLibrary.GetBuildConfiguration`) "Shipping")))