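; Base interactable actor that shows a selection outline and exposes empty hooks for being punched, chopped or grabbed.
; On BeginPlay it creates dynamic instances of the static mesh's overlay material and first material, hides the outline, then calls an empty ChildBeginPlay hook for subclasses.
; Select and deselect events toggle the overlay's Line Width parameter to show or hide the outline.
; IsSelected always returns false here.
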(event `/Game/BP_Select_Interface.SelectActor`
  (`self.ShowOutline`))

(event `/Game/BP_Select_Interface.DeselectActor`
  (`self.HideOutline`))

(event `ShowOutline`
  (bind _outlinematerial (`self.OutlineMaterial`))
  (`/Engine/EditorBlueprintResources/StandardMacros.IsValid` _outlinematerial
    (:`Is Valid`
      (`MaterialInstanceDynamic.SetScalarParameterValue` _outlinematerial "Line Width" 3.0))))

(event `ChildBeginPlay`)

(event `HideOutline`
  (bind _outlinematerial (`self.OutlineMaterial`))
  (`/Engine/EditorBlueprintResources/StandardMacros.IsValid` _outlinematerial
    (:`Is Valid`
      (`MaterialInstanceDynamic.SetScalarParameterValue` _outlinematerial "Line Width" 0.0))))

(event `self.ReceiveBeginPlay`
  (bind _staticmeshcomponent (`self.StaticMeshComponent`))
  (`|ExecutionSequence`
    (:`then_0`
      (bind _returnvalue (`KismetMaterialLibrary.CreateDynamicMaterialInstance` (`MeshComponent.GetOverlayMaterial` _staticmeshcomponent)))
      (bind _output_get (set `self.OutlineMaterial` _returnvalue))
      (`MeshComponent.SetOverlayMaterial` _staticmeshcomponent _output_get)
      (`self.HideOutline`))
    (:`then_1`
      (bind _returnvalue_2 (`KismetMaterialLibrary.CreateDynamicMaterialInstance` (`PrimitiveComponent.GetMaterial` _staticmeshcomponent 0)))
      (bind _output_get_2 (set `self.MainMaterial` _returnvalue_2))
      (`PrimitiveComponent.SetMaterial` _staticmeshcomponent 0 _output_get_2))
    (:`then_2`
      (`self.ChildBeginPlay`))))

(event `GetPunched`
  (params (HitComponent :type "PrimitiveComponent Object Reference")))

(event `GetChopped`
  (params (HitComponent :type "PrimitiveComponent Object Reference")))

(event `GetGrabbed`
  (params (HitComponent :type "PrimitiveComponent Object Reference")))

(fn `IsSelected`
  (returns (IsSelected :type Boolean))
  (return false))

(fn `UserConstructionScript`)