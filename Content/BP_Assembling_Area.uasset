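; Assembly spot where a loose ingredient becomes the base of a food combo.
; When an ingredient enters the free trigger, it is destroyed and replaced by a BP_Interactable_Food_Combo that inherits its item data and contamination state.
; An entering combo simply claims the spot.
; While occupied, the plate is hidden without collision, and it returns when a combo leaves the trigger.
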(event `self.AssembleTrigger.OnComponentBeginOverlap`
  (params (OverlappedComponent :type "PrimitiveComponent Object Reference") (OtherActor :type "Actor Object Reference") (OtherComp :type "PrimitiveComponent Object Reference") (OtherBodyIndex :type Integer) (bFromSweep :type Boolean) (SweepResult :type "HitResult Structure (by ref)"))
  (bind _returnvalue (`GameplayStatics.GetObjectClass` OtherActor))
  (if (or (== _returnvalue "/Game/BP_Interactable_Ingredient_Actor.BP_Interactable_Ingredient_Actor_C") (== _returnvalue "/Game/BP_Interactable_Food_Combo.BP_Interactable_Food_Combo_C"))
    (if (not (`self.IsOccupied`))
      (bind _asbp_interactable_ingredient_actor (cast `/Game/BP_Interactable_Ingredient_Actor` OtherActor)
        (:`then`
          (bind _output_get (set `self.ComboDataStart` (`/Game/BP_Interactable_Ingredient_Actor.ItemData` _asbp_interactable_ingredient_actor)))
          (bind _output_get_2 (set `self.ComboContaminationStart` (`/Game/BP_Interactable_Ingredient_Actor.IsContaminated` _asbp_interactable_ingredient_actor)))
          (`self.K2_DestroyActor` _asbp_interactable_ingredient_actor)
          (`|SpawnActorFromClass` "/Game/BP_Interactable_Food_Combo.BP_Interactable_Food_Combo_C" (`SceneComponent.K2_GetComponentToWorld` (`self.AssembleTrigger`)) "AdjustIfPossibleButAlwaysSpawn" "MultiplyWithRoot" null _output_get _output_get_2 null)
          (bind _output_get_3 (set `self.IsOccupied` true))
          (`self.TogglePlate` _output_get_3))
        (:`CastFailed`
          (cast `/Game/BP_Interactable_Food_Combo` OtherActor)
          (bind _output_get_4 (set `self.IsOccupied` true))
          (`self.TogglePlate` _output_get_4))))))

(event `self.AssembleTrigger.OnComponentEndOverlap`
  (params (OverlappedComponent :type "PrimitiveComponent Object Reference") (OtherActor :type "Actor Object Reference") (OtherComp :type "PrimitiveComponent Object Reference") (OtherBodyIndex :type Integer))
  (if (== (`GameplayStatics.GetObjectClass` OtherActor) "/Game/BP_Interactable_Food_Combo.BP_Interactable_Food_Combo_C")
    (bind _output_get (set `self.IsOccupied` false))
    (`self.TogglePlate` _output_get)))

(event `TogglePlate`
  (params (IsHidden :type Boolean))
  (bind _plate (`self.Plate`))
  (`SceneComponent.SetHiddenInGame` _plate IsHidden false)
  (if IsHidden
    (`PrimitiveComponent.SetCollisionEnabled` _plate "NoCollision")
    (else
      (`PrimitiveComponent.SetCollisionEnabled` _plate "QueryAndPhysics"))))

(fn `UserConstructionScript`)