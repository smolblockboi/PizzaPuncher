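; A data-driven interactable ingredient actor that can be grabbed, chopped, punched and contaminated, with mesh and rules taken from its ItemData.
; Each valid chop or punch spawns copies carrying the ChopInto or PunchInto data, flagged against further modification, and destroys the original once its hit count is reached.
; Tick accumulates contamination exposure until a threshold, driving a material parameter and a camera-facing stink bar widget above the mesh.
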(event `GotContaminated`
  (bind _mainmaterial (`self.MainMaterial`))
  (`MaterialInstanceDynamic.SetScalarParameterValue` _mainmaterial "Contamination" 1.0)
  (`MaterialInstanceDynamic.K2_GetScalarParameterValue` _mainmaterial "Contamination"))

(event `self.ReceiveTick`
  (params (DeltaSeconds :type "Float (single-precision)"))
  (bind _stinkywidget (`self.StinkyWidget`))
  (`SceneComponent.K2_SetRelativeLocation` _stinkywidget (`KismetMathLibrary.MakeVector` 0.0 0.0 (.z (`.Max` (`StaticMeshComponent.GetLocalBounds` (`self.StaticMeshComponent`))))) false true)
  (`SceneComponent.K2_SetWorldRotation` _stinkywidget (`KismetMathLibrary.FindLookAtRotation` (`self.K2_GetActorLocation` self) (`PlayerCameraManager.GetCameraLocation` (`GameplayStatics.GetPlayerCameraManager` 0))) false false)
  (if (and (`self.BeingContaminated`) (not (`self.IsContaminated`)))
    (bind _output_get (set `self.ContaminationTracked` (+ (`self.ContaminationTracked`) DeltaSeconds)))
    (`MaterialInstanceDynamic.SetScalarParameterValue` (`self.MainMaterial`) "Contamination" _output_get)
    (bind _w_stinky_bar (`self.GetStinkyWidget`))
    (set `/Game/PP_Items/W_Stinky_Bar.StinkTime` _output_get _w_stinky_bar)
    (if (>= _output_get 5.0)
      (set `self.IsContaminated` true)
      (`self.GotContaminated`))))

(event `ChangeData`
  (params (NewData :type "/Game/PP_Items/DA_Item_Data Object Reference"))
  (bind _output_get (set `self.ItemData` NewData))
  (bind _itemmesh (`/Game/PP_Items/DA_Item_Data.ItemMesh` _output_get))
  (`/Engine/EditorBlueprintResources/StandardMacros.IsValid` _itemmesh
    (:`Is Valid`
      (`StaticMeshComponent.SetStaticMesh` (`self.StaticMeshComponent`) _itemmesh))))

(event `self.GetChopped`
  (params (HitComponent :type "PrimitiveComponent Object Reference"))
  (bind _itemdata (`self.ItemData`))
  ; Chopped
  (if (`self.IsAlreadyModified`)
    _
    (elif (`KismetSystemLibrary.IsValid` _itemdata)
      (if (`/Game/PP_Items/DA_Item_Data.Choppable` _itemdata)
        (`GameplayStatics.PlaySoundAtLocation` (`AudioComponent.Sound` (`self.ChoppedAudio`)) (`SceneComponent.K2_GetComponentLocation` HitComponent) (struct) 1.0 1.0 0.0 null null null null)
        (bind _result (`/Engine/EditorBlueprintResources/StandardMacros.IncrementInt` (`self.ChopsTracked`))
          (:`  `
            (for _index (range (`self.SpawnAmount`))
              (bind _result_2 (`self.GetSpawnTransform` _index))
              (bind _returnvalue (`|SpawnActorFromClass` "BP_Interactable_Ingredient_Actor_C" _result_2 "AdjustIfPossibleButAlwaysSpawn" "MultiplyWithRoot" null (`/Game/PP_Items/DA_Item_Data.ChopInto` (`self.ItemData`)) null))
              (set `/Game/BP_Interactable_Ingredient_Actor.IsChopped` true _returnvalue))
            (if (>= _result (`/Game/PP_Items/DA_Item_Data.ChopsRemaining` (`self.ItemData`)))
              (`self.K2_DestroyActor`))))))))

(event `self.GetPunched`
  (params (HitComponent :type "PrimitiveComponent Object Reference"))
  (bind _itemdata (`self.ItemData`))
  ; Punched
  (if (`self.IsAlreadyModified`)
    _
    (elif (`KismetSystemLibrary.IsValid` _itemdata)
      (if (`/Game/PP_Items/DA_Item_Data.Punchable` _itemdata)
        (`GameplayStatics.PlaySoundAtLocation` (`AudioComponent.Sound` (`self.PunchedAudio`)) (`SceneComponent.K2_GetComponentLocation` HitComponent) (struct) 1.0 1.0 0.0 null null null null)
        (bind _result (`/Engine/EditorBlueprintResources/StandardMacros.IncrementInt` (`self.PunchesTracked`))
          (:`  `
            (for _ (range (`self.SpawnAmount`))
              (bind _returnvalue (`|SpawnActorFromClass` "BP_Interactable_Ingredient_Actor_C" (`self.GetTransform` self) "AdjustIfPossibleButAlwaysSpawn" "MultiplyWithRoot" self (`/Game/PP_Items/DA_Item_Data.PunchInto` (`self.ItemData`)) null))
              (set `/Game/BP_Interactable_Ingredient_Actor.IsPunched` true _returnvalue))
            (if (>= _result (`/Game/PP_Items/DA_Item_Data.PunchesRemaining` (`self.ItemData`)))
              (`self.K2_DestroyActor`))))))))

(event `self.GetGrabbed`
  (params (HitComponent :type "PrimitiveComponent Object Reference"))
  (`AudioComponent.Play` (`self.GrabbedAudio`) 0.0))

(fn `GetSpawnTransform`
  (params (HeightOffset :type Integer))
  (returns (Result :type "Transform Structure"))
  (bind (_returnvalue_location _returnvalue_rotation _returnvalue_scale) (`KismetMathLibrary.BreakTransform` (`self.GetTransform` self)))
  (return (`KismetMathLibrary.MakeTransform` (+ (+ _returnvalue_location (`KismetMathLibrary.MakeVector` 0.0 0.0 (* (.z (`.Max` (`StaticMeshComponent.GetLocalBounds` (`self.StaticMeshComponent`)))) 0.5))) (`KismetMathLibrary.MakeVector` 0.0 0.0 (* HeightOffset 15))) _returnvalue_rotation _returnvalue_scale)))

(fn `GetStinkyWidget`
  (returns (`W Stinky Bar` :type "/Game/PP_Items/W_Stinky_Bar Object Reference"))
  (bind _asw_stinky_bar (cast `/Game/PP_Items/W_Stinky_Bar` (`WidgetComponent.GetWidget` (`self.StinkyWidget`))))
  (return _asw_stinky_bar))

(fn `IsAlreadyModified`
  (returns (Result :type Boolean))
  (return (or (`self.IsChopped`) (`self.IsPunched`))))

(fn `UserConstructionScript`
  (bind _itemmesh (`/Game/PP_Items/DA_Item_Data.ItemMesh` (`self.ItemData`)))
  (`parent.UserConstructionScript`)
  (`/Engine/EditorBlueprintResources/StandardMacros.IsValid` _itemmesh
    (:`Is Valid`
      (`StaticMeshComponent.SetStaticMesh` (`self.StaticMeshComponent`) _itemmesh))))